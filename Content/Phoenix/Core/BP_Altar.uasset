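; BP_Altar is an interactable level exit that sends the player to the next level once the wave manager reports all waves cleared.
; On BeginPlay it caches BP_WaveManager; the Sphere overlap enables input for the player character and shows an interact widget if waves are cleared.
; Pressing E in range activates the Flame, removes the prompt and, after a short delay, opens the level named by NextLevelName.
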(event `self.ReceiveBeginPlay`
  (bind _returnvalue (`GameplayStatics.GetActorOfClass` "/Game/Phoenix/Core/BP_WaveManager.BP_WaveManager_C"))
  (bind _asbp_wave_manager (cast `/Game/Phoenix/Core/BP_WaveManager` _returnvalue))
  (set `self.WaveManagerRef` _asbp_wave_manager))

(event `self.Sphere.OnComponentBeginOverlap`
  (params (OverlappedComponent :type "PrimitiveComponent Object Reference") (OtherActor :type "Actor Object Reference") (OtherComp :type "PrimitiveComponent Object Reference") (OtherBodyIndex :type Integer) (bFromSweep :type Boolean) (SweepResult :type "HitResult Structure (by ref)"))
  (bind _returnvalue (`GameplayStatics.GetPlayerController` 0))
  (cast `/Game/ThirdPerson/Blueprints/BP_ThirdPersonCharacter` OtherActor)
  (set `self.bPlayerInRange ` true)
  (`self.EnableInput` _returnvalue)
  (if (`/Game/Phoenix/Core/BP_WaveManager.bWavesCleared` (`self.WaveManagerRef`))
    (bind _returnvalue_2 (`|CreateWidget` "/Game/Phoenix/UI/WBP_Interact.WBP_Interact_C" _returnvalue))
    (`UserWidget.AddToViewport` _returnvalue_2 0)
    (set `self.PromptWidget` _returnvalue_2)))

(event `self.Sphere.OnComponentEndOverlap`
  (params (OverlappedComponent :type "PrimitiveComponent Object Reference") (OtherActor :type "Actor Object Reference") (OtherComp :type "PrimitiveComponent Object Reference") (OtherBodyIndex :type Integer))
  (bind _promptwidget (`self.PromptWidget`))
  (cast `/Game/ThirdPerson/Blueprints/BP_ThirdPersonCharacter` OtherActor)
  (set `self.bPlayerInRange ` false)
  (`self.DisableInput` (`GameplayStatics.GetPlayerController` 0))
  (`/Engine/EditorBlueprintResources/StandardMacros.IsValid` _promptwidget
    (:`Is Valid`
      (`Widget.RemoveFromParent` _promptwidget))))

(event `Key|E`
  (params (Key :type "Key Structure"))
  (:`Pressed`
    (if (and (`self.bPlayerInRange `) (`/Game/Phoenix/Core/BP_WaveManager.bWavesCleared` (`self.WaveManagerRef`)))
      (`self.DisableInput` (`GameplayStatics.GetPlayerController` 0))
      (`ActorComponent.Activate` (`self.Flame`) true)
      (`Widget.RemoveFromParent` (`self.PromptWidget`))
      (`KismetSystemLibrary.Delay` 1.5)
      (`GameplayStatics.OpenLevel` (`self.NextLevelName`)))))

(fn `UserConstructionScript`)