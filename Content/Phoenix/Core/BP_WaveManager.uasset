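; Wave manager actor that runs three scripted waves of shadow and ice enemies, the last one mixed.
; On BeginPlay it caches the level's TargetPoints, starts the first wave and sets a looping one-second timer, apparently to poll CheckWaveComplete.
; That check starts the next wave once no BP_EnemyIce or BP_EnemyBase actors remain.
; StartWave spawns enemies at the first three points, or sets WavesCleared after the final wave.
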(event `self.ReceiveBeginPlay`
  (bind _outactors (`GameplayStatics.GetAllActorsOfClass` "/Script/Engine.TargetPoint"))
  (set `self.SpawnPoints` _outactors)
  (`self.StartWave`)
  (`KismetSystemLibrary.K2_SetTimerDelegate` (`|CreateDelegate` :!event `CheckWaveComplete`) 1.0 true))

(event `CheckWaveComplete`
  (bind _outactors (`GameplayStatics.GetAllActorsOfClass` "/Game/Phoenix/Enemies/BP_EnemyIce.BP_EnemyIce_C"))
  (bind _outactors_2 (`GameplayStatics.GetAllActorsOfClass` "/Game/Phoenix/Enemies/BP_EnemyBase.BP_EnemyBase_C"))
  (if (== (+ (`KismetArrayLibrary.Array_Length` _outactors) (`KismetArrayLibrary.Array_Length` _outactors_2)) 0)
    (`self.StartWave`)))

(event `StartWave`
  (if (>= (`self.CurrentWave `) 3)
    (set `self.bWavesCleared` true)
    (else
      (bind _result (`/Engine/EditorBlueprintResources/StandardMacros.IncrementInt` (`self.CurrentWave `))
        (:`  `
          (bind _output_get (set `self.CurrentWave ` _result))
          (switch `int` _output_get
            (:`1`
              (`self.SpawnEnemy` (`self.ShadowEnemyClass `) (`|GetArrayItem` (`self.SpawnPoints`)))
              (`self.SpawnEnemy` (`self.ShadowEnemyClass `) (`|GetArrayItem` (`self.SpawnPoints`) 1))
              (`self.SpawnEnemy` (`self.ShadowEnemyClass `) (`|GetArrayItem` (`self.SpawnPoints`) 2)))
            (:`2`
              (`self.SpawnEnemy` (`self.IceEnemyClass`) (`|GetArrayItem` (`self.SpawnPoints`)))
              (`self.SpawnEnemy` (`self.IceEnemyClass`) (`|GetArrayItem` (`self.SpawnPoints`) 1))
              (`self.SpawnEnemy` (`self.IceEnemyClass`) (`|GetArrayItem` (`self.SpawnPoints`) 2)))
            (:`3`
              (`self.SpawnEnemy` (`self.IceEnemyClass`) (`|GetArrayItem` (`self.SpawnPoints`)))
              (`self.SpawnEnemy` (`self.ShadowEnemyClass `) (`|GetArrayItem` (`self.SpawnPoints`) 1))
              (`self.SpawnEnemy` (`self.IceEnemyClass`) (`|GetArrayItem` (`self.SpawnPoints`) 2)))))))))

(fn `SpawnEnemy`
  (params (EnemyClass :type "Actor Class Reference") (SpawnPoint :type "Actor Object Reference"))
  (`|SpawnActorFromClass` EnemyClass (`self.GetTransform` SpawnPoint) "AdjustIfPossibleButAlwaysSpawn" "MultiplyWithRoot" null null))

(fn `UserConstructionScript`)