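; Fire projectile actor that deals fire damage to actors it hits and expires after a short lifespan.
; Sphere collision hits skip the instigator, pass fixed damage to the other actor's HealthComponent if present, and destroy the projectile on any other valid actor.
; BeginPlay calls IgnoreActorWhenMoving on the instigator with ShouldIgnore false, so only the hit check excludes the shooter.
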(event `self.ReceiveBeginPlay`
  (`self.SetLifeSpan` 3.0)
  (`PrimitiveComponent.IgnoreActorWhenMoving` (`self.SphereCollision`) (`self.GetInstigator`) false))

(event `self.SphereCollision.OnComponentHit`
  (params (HitComponent :type "PrimitiveComponent Object Reference") (OtherActor :type "Actor Object Reference") (OtherComp :type "PrimitiveComponent Object Reference") (NormalImpulse :type "Vector Structure") (Hit :type "HitResult Structure (by ref)"))
  (bind _returnvalue (`self.GetComponentByClass` OtherActor "/Script/PhoenixAscendant.HealthComponent"))
  (`/Engine/EditorBlueprintResources/StandardMacros.IsValid` OtherActor
    (:`Is Valid`
      (if (not (== OtherActor (`self.GetInstigator`)))
        (`/Engine/EditorBlueprintResources/StandardMacros.IsValid` _returnvalue
          (:`Is Valid`
            (`HealthComponent.ApplyDamage` _returnvalue 10.0 "Fire")
            (`self.K2_DestroyActor`))
          (:`Is Not Valid`
            (`self.K2_DestroyActor`)))))))

(fn `UserConstructionScript`)